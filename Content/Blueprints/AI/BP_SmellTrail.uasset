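; BP_SmellTrail is an AI smell trail actor that models scent drifting on the wind as a spline.
; A looping five-second timer appends the actor's location, then removes index MaxPoints-1 once the count reaches MaxPoints, so a full trail drops the new point.
; A faster looping timer shifts every point except the last by the wind direction from the GameMode's WeatherManager.
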(event `self.ReceiveBeginPlay`
  (bind _reference (message `/Game/ThirdPerson/Blueprints/BPI_Gamemode.GetReference(Gamemode)` (`GameplayStatics.GetGameMode`)))
  (set `self.Weather Manager` (`/Game/ThirdPerson/Blueprints/BP_ThirdPersonGameMode.WeatherManager` _reference))
  (`self.Run`))

(event `Run`
  (`KismetSystemLibrary.K2_SetTimer` null "UpdateSpline" 0.1 true)
  (`KismetSystemLibrary.K2_SetTimer` null "AddPoint" 5.0 true))

(fn `AddPoint`
  (`SplineComponent.AddSplinePoint` (`self.Spline`) (`self.K2_GetActorLocation`) "World" true)
  (if (>= (`SplineComponent.GetNumberOfSplinePoints` (`self.Spline`)) (`self.MaxPoints`))
    (`SplineComponent.RemoveSplinePoint` (`self.Spline`) (- (`self.MaxPoints`) 1) true)))

(fn `UpdateSpline`
  (bind _spline (`self.Spline`))
  (for _index (range (+ (- (`SplineComponent.GetNumberOfSplinePoints` (`self.Spline`)) 2) 1))
    (`SplineComponent.SetLocationAtSplinePoint` _spline _index (+ (`SplineComponent.GetLocationAtSplinePoint` _spline _index "World") (`/Game/Blueprints/Environment/Weather/WeatherManager.GetWind` (`self.Weather Manager`))) "World" true)))

(fn `UserConstructionScript`)