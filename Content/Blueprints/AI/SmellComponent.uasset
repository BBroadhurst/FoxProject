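; SmellComponent is an AI component that gives its owning actor a coloured Niagara smell trail that responds to wind.
; On BeginPlay it adds a Niagara component to the owner, assigns the trail system and colour, and gets the WeatherManager through the game mode.
; A fast looping timer then reads the wind from the WeatherManager and feeds its direction into the trail's WindDirection variable.
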(event `self.ReceiveBeginPlay`
  (bind _returnvalue (`|AddComponentByClass` :`self` (`self.GetOwner`) :`Class` "/Script/Niagara.NiagaraComponent"))
  (set `self.Trail` _returnvalue)
  (`NiagaraComponent.SetAsset` _returnvalue "/Game/AI/Effects/N_Trail_EM_System.N_Trail_EM_System" true)
  (`NiagaraComponent.SetNiagaraVariableLinearColor` (`self.Trail`) "Colour" (`self.Colour`))
  (bind _reference (message `/Game/ThirdPerson/Blueprints/BPI_Gamemode.GetReference(Gamemode)` (`GameplayStatics.GetGameMode`)))
  (bind _output_get (set `self.Gamemode` _reference))
  (set `self.Weather Manager` (`/Game/ThirdPerson/Blueprints/BP_ThirdPersonGameMode.WeatherManager` _output_get))
  (`self.Run`))

(event `Run`
  (`KismetSystemLibrary.K2_SetTimerDelegate` (delegate `Update`) 0.05 true))

(event `Update`
  (bind _winddirection (`/Game/Blueprints/Environment/Weather/WeatherManager.GetWind` (`self.Weather Manager`)))
  (`NiagaraComponent.SetNiagaraVariableVec3` (`self.Trail`) "WindDirection" _winddirection))