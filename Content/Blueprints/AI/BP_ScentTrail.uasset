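; BP_ScentTrail is an AI scent trail that records its actor's location as a wind-blown spline.
; Looping timers append a point every few seconds, trimming the oldest at MaxPoints, and frequently shift all but the newest by the WeatherManager's wind direction.
; Query functions return the nearest point and distance along the trail for a world location.
; A spline mesh stretched between the trail's ends is marked for deletion.
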(event `self.ReceiveBeginPlay`
  (bind _reference (message `/Game/ThirdPerson/Blueprints/BPI_Gamemode.GetReference(Gamemode)` (`GameplayStatics.GetGameMode`)))
  (set `self.Weather Manager` (`/Game/ThirdPerson/Blueprints/BP_ThirdPersonGameMode.WeatherManager` _reference))
  (`self.Run`))

(event `Run`
  (`KismetSystemLibrary.K2_SetTimer` null "UpdateSpline" 0.1 true)
  (`KismetSystemLibrary.K2_SetTimer` null "AddPoint" 5.0 true))

(fn `AddPoint`
  (`SplineComponent.AddSplinePoint` (`self.Spline`) (`self.K2_GetActorLocation`) "World" true)
  (if (>= (`SplineComponent.GetNumberOfSplinePoints` (`self.Spline`)) (`self.MaxPoints`))
    (`SplineComponent.RemoveSplinePoint` (`self.Spline`) 0 true)))

(fn `GetDistanceAtLocation`
  (params (WorldLocation :type "Vector Structure (by ref)"))
  (returns (ReturnValue :type "Float (single-precision)"))
  (bind _spline (`self.Spline`))
  (return (`SplineComponent.GetDistanceAlongSplineAtSplineInputKey` _spline (`SplineComponent.FindInputKeyClosestToWorldLocation` _spline WorldLocation))))

(fn `GetNearestPoint`
  (params (WorldLocation :type "Vector Structure (by ref)"))
  (returns (ReturnValue :type Integer))
  (return (`KismetMathLibrary.Round` (`SplineComponent.FindInputKeyClosestToWorldLocation` (`self.Spline`) WorldLocation))))

(fn `GetReference_ScentTrail`
  (returns (Reference :type "/Game/Blueprints/AI/BP_ScentTrail Object Reference"))
  (return self))

(fn `UpdateSpline`
  (bind _spline (`self.Spline`))
  (bind _spline_2 (`self.Spline`))
  (bind _returnvalue (- (`SplineComponent.GetNumberOfSplinePoints` (`self.Spline`)) 1))
  (`|ExecutionSequence`
    (:`then_0`
      (for _index (range (+ (- (`SplineComponent.GetNumberOfSplinePoints` (`self.Spline`)) 2) 1))
        (`SplineComponent.SetLocationAtSplinePoint` _spline_2 _index (+ (`SplineComponent.GetLocationAtSplinePoint` _spline_2 _index "World") (`/Game/Blueprints/Environment/Weather/WeatherManager.GetWind` (`self.Weather Manager`))) "World" true)))
    (:`then_1`
      ;[1 0 0] *DELETE*
      (`SplineMeshComponent.SetStartAndEnd` (`self.SplineMesh`) (`SplineComponent.GetLocationAtSplinePoint` _spline 0 "World") (`SplineComponent.GetTangentAtSplinePoint` _spline 0 "World") (`SplineComponent.GetLocationAtSplinePoint` _spline _returnvalue "World") (`SplineComponent.GetTangentAtSplinePoint` _spline _returnvalue "World") true))))

(fn `UserConstructionScript`)