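; Scent trail that records its actor's path as a spline and lets it drift with the wind.
; A slow looping timer adds points at the actor's location, trimming the oldest at MaxPoints, while a fast one shifts all but the newest by the WeatherManager's wind vector.
; Helper functions return the closest point, distance or location along the trail.
; Spline meshes are built at construction; their runtime rebuild is never called.
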(event `self.ReceiveBeginPlay`
  (bind _reference (message `/Game/ThirdPerson/Blueprints/BPI_Gamemode.GetReference(Gamemode)` (`GameplayStatics.GetGameMode`)))
  (set `self.Weather Manager` (`/Game/ThirdPerson/Blueprints/BP_ThirdPersonGameMode.WeatherManager` _reference))
  (`self.Run`))

(event `Run`
  (`KismetSystemLibrary.K2_SetTimer` null "UpdateSpline" 0.1 true)
  (`KismetSystemLibrary.K2_SetTimer` null "AddPoint" 5.0 true))

(fn `AddPoint`
  (`SplineComponent.AddSplinePoint` (`self.Spline`) (`self.K2_GetActorLocation`) "World" true)
  (if (>= (`SplineComponent.GetNumberOfSplinePoints` (`self.Spline`)) (`self.MaxPoints`))
    (`SplineComponent.RemoveSplinePoint` (`self.Spline`) 0 true)))

(fn `ClearSplineMeshes`
  (for _array_element (`self.Splinemeshs`)
    (`ActorComponent.K2_DestroyComponent` _array_element)))

(fn `FindClosestPointToActor`
  (params (Actor :type "Actor Object Reference"))
  (returns (ReturnValue :type "Vector Structure"))
  (return (`SplineComponent.FindLocationClosestToWorldLocation` (`self.Spline`) (`self.K2_GetActorLocation` Actor) "World")))

(fn `GetDistanceAtLocation`
  (params (WorldLocation :type "Vector Structure (by ref)"))
  (returns (ReturnValue :type "Float (single-precision)"))
  (bind _spline (`self.Spline`))
  (return (`SplineComponent.GetDistanceAlongSplineAtSplineInputKey` _spline (`SplineComponent.FindInputKeyClosestToWorldLocation` _spline WorldLocation))))

(fn `GetNearestPoint`
  (params (WorldLocation :type "Vector Structure (by ref)"))
  (returns (ReturnValue :type Integer))
  (return (`KismetMathLibrary.Round` (`SplineComponent.FindInputKeyClosestToWorldLocation` (`self.Spline`) WorldLocation))))

(fn `GetReference_ScentTrail`
  (returns (Reference :type "/Game/Blueprints/Components/Smell_Comp/BP_ScentTrail Object Reference"))
  (return self))

(fn `SplineMesh`
  (bind _spline (`self.Spline`))
  (for _index (range 1 (+ (`SplineComponent.GetNumberOfSplinePoints` (`self.Spline`)) 1))
    (bind _returnvalue (`AddComponent|NODE_AddSplineMeshComponent-4`))
    (bind (_location _tangent) (`SplineComponent.GetLocationAndTangentAtSplinePoint` _spline _index "World"))
    (bind (_location_2 _tangent_2) (`SplineComponent.GetLocationAndTangentAtSplinePoint` _spline (+ _index 1) "World"))
    (`SplineMeshComponent.SetStartAndEnd` _returnvalue _location _tangent _location_2 _tangent_2 true)
    (`KismetArrayLibrary.Array_Add` (`self.Splinemeshs`) _returnvalue)))

(fn `UpdateSpline`
  (bind _spline (`self.Spline`))
  (`|ExecutionSequence`
    (:`then_0`
      (for _index (range (+ (- (`SplineComponent.GetNumberOfSplinePoints` (`self.Spline`)) 2) 1))
        (`SplineComponent.SetLocationAtSplinePoint` _spline _index (+ (`SplineComponent.GetLocationAtSplinePoint` _spline _index "World") (`/Game/Blueprints/Environment/Weather/WeatherManager.GetWind` (`self.Weather Manager`))) "World" true)))))

(fn `UserConstructionScript`
  (bind _spline (`self.Spline`))
  (for _index (range 1 (+ (`SplineComponent.GetNumberOfSplinePoints` (`self.Spline`)) 1))
    (bind _returnvalue (`AddComponent|NODE_AddSplineMeshComponent-2`))
    (bind (_location _tangent) (`SplineComponent.GetLocationAndTangentAtSplinePoint` _spline _index "World"))
    (bind (_location_2 _tangent_2) (`SplineComponent.GetLocationAndTangentAtSplinePoint` _spline (+ _index 1) "World"))
    (`SplineMeshComponent.SetStartAndEnd` _returnvalue _location _tangent _location_2 _tangent_2 true)))