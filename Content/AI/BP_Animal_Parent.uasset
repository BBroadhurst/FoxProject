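; Base Character Blueprint for AI animals, providing shared survival stats, movement speed and alert feedback.
; AddHunger and AddHydration raise their stat in the SAnimalStats struct, capped at the MaxStats value.
; SetSprint switches max walk speed between walk and sprint, and SetAlert toggles two alert widgets.
; A getter returns the animal itself, while GetBlackboard has no connected logic.
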(event `Set Alert`
  (params (Alerted :type Boolean))
  ;[1 1 1] Display Alert widget
  (`SceneComponent.SetVisibility` (`self.Widget`) Alerted false)
  (`SceneComponent.SetVisibility` (`self.Widget90`) Alerted false))

(fn `AddHunger`
  (params (Amount :type "Float (double-precision)"))
  (bind (_stats_health _stats_stamina _stats_hunger) (break `/Game/AI/Blueprint/S_AnimalStats` (`self.Stats`)))
  (bind (_stats_health_2 _stats_stamina_2 _stats_hunger_2 _stats_hydration _stats_fatigue) (break `/Game/AI/Blueprint/S_AnimalStats` (`self.Stats`)))
  (bind (_maxstats_health _maxstats_stamina _maxstats_hunger) (break `/Game/AI/Blueprint/S_AnimalStats` (`self.MaxStats`)))
  (bind (_stats_health_3 _stats_stamina_3 _stats_hunger_3 _stats_hydration_2 _stats_fatigue_2) (break `/Game/AI/Blueprint/S_AnimalStats` (`self.Stats`)))
  (bind _returnvalue (+ _stats_hunger Amount))
  ;[1 1 1] If resultant Hunger is less than Max hunger set Hunger as result.
  (if (not (> _returnvalue _maxstats_hunger))
    (set `self.Stats` (make `/Game/AI/Blueprint/S_AnimalStats` _stats_health_3 _stats_stamina_3 _returnvalue _stats_hydration_2 _stats_fatigue_2))
    (else
      ;[1 1 1] If resultant Hunger is Greater than Max Hunger set Hunger to Max.
      (set `self.Stats` (make `/Game/AI/Blueprint/S_AnimalStats` _stats_health_2 _stats_stamina_2 _maxstats_hunger _stats_hydration _stats_fatigue)))))

(fn `AddHydration`
  (params (Amount :type "Float (double-precision)"))
  (bind (_stats_health _stats_stamina _stats_hunger _stats_hydration) (break `/Game/AI/Blueprint/S_AnimalStats` (`self.Stats`)))
  (bind (_stats_health_2 _stats_stamina_2 _stats_hunger_2 _stats_hydration_2 _stats_fatigue) (break `/Game/AI/Blueprint/S_AnimalStats` (`self.Stats`)))
  (bind (_maxstats_health _maxstats_stamina _maxstats_hunger _maxstats_hydration) (break `/Game/AI/Blueprint/S_AnimalStats` (`self.MaxStats`)))
  (bind (_stats_health_3 _stats_stamina_3 _stats_hunger_3 _stats_hydration_3 _stats_fatigue_2) (break `/Game/AI/Blueprint/S_AnimalStats` (`self.Stats`)))
  (bind _returnvalue (+ _stats_hydration Amount))
  ;[1 1 1] If resultant Hunger is less than Max hunger set Hunger as result.
  (if (not (> _returnvalue _maxstats_hydration))
    (set `self.Stats` (make `/Game/AI/Blueprint/S_AnimalStats` _stats_health_3 _stats_stamina_3 _stats_hunger_3 _returnvalue _stats_fatigue_2))
    (else
      ;[1 1 1] If resultant Hunger is Greater than Max Hunger set Hunger to Max.
      (set `self.Stats` (make `/Game/AI/Blueprint/S_AnimalStats` _stats_health_2 _stats_stamina_2 _stats_hunger_2 _maxstats_hydration _stats_fatigue)))))

(fn `Get Reference (Animal)`
  (returns (Reference :type "/Game/AI/BP_Animal_Parent Object Reference"))
  (return self))

(fn `SetSprint`
  (params (Sprint :type Boolean))
  (bind _charactermovement (`self.CharacterMovement`))
  (if Sprint
    (set `CharacterMovementComponent.MaxWalkSpeed` (`self.SprintSpeed`) _charactermovement)
    (else
      (set `CharacterMovementComponent.MaxWalkSpeed` (`self.WalkSpeed`) _charactermovement))))

(fn `UserConstructionScript`)