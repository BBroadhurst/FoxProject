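; BP_AnimalPathSpline is an AI helper actor holding a short, rolling spline path for animals.
; SetStartAndEnd seeds two local-space points; AddPoint appends world-space points and trims the oldest, keeping at most four.
; After each append, IncreaseNewTangent aims to scale X/Y tangents by SplineMulipltyer, but indexes at the point count, one past the last point.
; A getter returns the actor itself.
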(fn `AddPoint`
  (params (`Point Position` :type "Vector Structure"))
  (bind _spline (`self.Spline`))
  (`SplineComponent.AddSplinePoint` _spline `Point Position` "World" true)
  (`self.IncreaseNewTangent`)
  (while (>= (`SplineComponent.GetNumberOfSplinePoints` _spline) 5)
    (`SplineComponent.RemoveSplinePoint` (`self.Spline`) 0 true)))

(fn `GetReference_AnimalPathSpline`
  (returns (Reference :type "/Game/AI/Blueprint/BP_AnimalPathSpline Object Reference"))
  (return self))

(fn `IncreaseNewTangent`
  (bind _spline (`self.Spline`))
  (bind _splinemulipltyer (`self.SplineMulipltyer`))
  (bind _returnvalue (- (`SplineComponent.GetNumberOfSplinePoints` _spline) 0))
  (bind (_returnvalue_x _returnvalue_y _returnvalue_z) (`KismetMathLibrary.BreakVector` (`SplineComponent.GetArriveTangentAtSplinePoint` _spline _returnvalue "Local")))
  (bind (_returnvalue_x_2 _returnvalue_y_2 _returnvalue_z_2) (`KismetMathLibrary.BreakVector` (`SplineComponent.GetLeaveTangentAtSplinePoint` _spline _returnvalue "Local")))
  (`SplineComponent.SetTangentsAtSplinePoint` _spline (- (`SplineComponent.GetNumberOfSplinePoints` _spline) 0) (`KismetMathLibrary.MakeVector` (* _returnvalue_x _splinemulipltyer) (* _returnvalue_y _splinemulipltyer) _returnvalue_z) (`KismetMathLibrary.MakeVector` (* _returnvalue_x_2 _splinemulipltyer) (* _returnvalue_y_2 _splinemulipltyer) _returnvalue_z_2) "Local" true))

(fn `SetStartAndEnd`
  (params (Start :type "Vector Structure") (End :type "Vector Structure"))
  (`SplineComponent.SetSplinePoints` (`self.Spline`) (`|MakeArray` Start End) "Local" true))

(fn `UserConstructionScript`)